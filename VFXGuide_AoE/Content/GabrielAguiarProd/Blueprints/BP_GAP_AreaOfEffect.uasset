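; Area-of-effect VFX actor that plays a configurable Niagara system at an offset location, then destroys itself after a delay.
; The construction script assigns the system and pushes Scale as both vector and float parameters.
; Impact delay and optional two-colour overrides apply only when ImpactDelay is above zero.
; BeginPlay reassigns the system, offsets the actor by Location, sets its Rotation and starts the destroy timer.
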(event `self.ReceiveBeginPlay`
  (`self.SpawnAoE`)
  (`KismetSystemLibrary.Delay` (`self.DelayBeforeDestroying`))
  (`self.K2_DestroyActor`))

(event `SpawnAoE`
  (`NiagaraComponent.SetAsset` (`self.AreaOfEffectNiagara`) (`self.VFXAreaOfEffectNiagara`))
  (`self.K2_SetActorLocationAndRotation` (+ (`self.K2_GetActorLocation`) (`self.Location`)) (`self.Rotation`)))

(fn `UserConstructionScript`
  (bind _scale (`self.Scale`))
  (bind _areaofeffectniagara (`self.AreaOfEffectNiagara`))
  (bind _impactdelay (`self.ImpactDelay`))
  (if (`KismetSystemLibrary.IsValid` (`self.VFXAreaOfEffectNiagara`))
    (`NiagaraComponent.SetAsset` _areaofeffectniagara (`self.VFXAreaOfEffectNiagara`))
    (`NiagaraComponent.SetVariableVec3` _areaofeffectniagara "Scale" _scale)
    (`NiagaraComponent.SetVariableFloat` _areaofeffectniagara "Scale" (.x _scale))
    (if (> _impactdelay 0.0)
      (`NiagaraComponent.SetVariableFloat` _areaofeffectniagara "ImpactDelay" _impactdelay)
      (if (`self.ChangeColour1`)
        (`NiagaraComponent.SetVariableLinearColor` (`self.AreaOfEffectNiagara`) "Colour1" (`self.Colour1`)))
      (if (`self.ChangeColour2`)
        (`NiagaraComponent.SetVariableLinearColor` (`self.AreaOfEffectNiagara`) "Colour2" (`self.Colour2`))))))